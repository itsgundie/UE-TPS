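; Test variant of a TPS pickup item whose data and color are supplied from outside.
; SetPickupData stores the given pickup data and test color, then calls PickupInit.
; GeneratePickupColor returns that stored color, so the pickup's color is set by the caller.
; BeginPlay, overlap and Tick are unused disabled stubs, and the construction script only calls the parent.
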(event `SetPickupData`
  (params (PickupData :type "PickupData Structure") (PickupColor :type "LinearColor Structure"))
  (set `self.PickupData` PickupData)
  (set `self.Test Pickup Color` PickupColor)
  (`self.PickupInit`))

(fn `GeneratePickupColor`
  (returns (GeneratedPickupColor :type "LinearColor Structure"))
  (return (`self.Test Pickup Color`)))

(fn `UserConstructionScript`
  (`parent.UserConstructionScript`))